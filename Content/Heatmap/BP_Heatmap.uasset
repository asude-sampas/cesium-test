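; BP_Heatmap is a heatmap actor that paints heat splats into a runtime render target.
; The construction script creates a dynamic instance of M_HeatSplat, which DrawToRenderTarget feeds with size, strength and position before drawing it.
; Position comes from transforming the world location into the PositionGatheringPlane's local space and dividing by Resolution.
; Tick does nothing, and the player check and test draw are disconnected.
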(event Custom|DrawToRenderTarget
  (params (Location :type Vector) (Strength :type Float%20%28double-precision%29) (Size :type Float%20%28double-precision%29))
  (bind _mid_heatsplat (Variables|Default|GetMID_Heatsplat))
  (Rendering|Material|SetScalarParameterValue _mid_heatsplat "Size" Size :!class /Script/Engine.MaterialInstanceDynamic)
  (Rendering|Material|SetScalarParameterValue _mid_heatsplat "Strength" Strength :!class /Script/Engine.MaterialInstanceDynamic)
  (Rendering|Material|SetVectorParameterValue _mid_heatsplat "Position" (Math|Conversions|ToLinearColor(Vector) (/ (Math|Transform|TransformLocation (Math|Transform|InvertTransform (Transformation|GetWorldTransform (Variables|Default|GetPositionGatheringPlane))) Location) (Variables|Default|GetResolution))) :!class /Script/Engine.MaterialInstanceDynamic)
  (Rendering|DrawMaterialtoRenderTarget (Variables|Default|GetRenderTargetRuntime) _mid_heatsplat))

(event EventTick
  (params (DeltaSeconds :type Float%20%28single-precision%29)))

(fn ConstructionScript
  (bind _returnvalue (Rendering|Material|CreateDynamicMaterialInstance "/Game/Heatmap/M_HeatSplat.M_HeatSplat" "None" "None" :!class /Script/Engine.KismetMaterialLibrary))
  (Variables|Default|SetMID_Heatsplat _returnvalue))